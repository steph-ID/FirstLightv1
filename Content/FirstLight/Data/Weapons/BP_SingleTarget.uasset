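; BP_SingleTarget is a weapon hit actor that applies damage and stun to AI characters through the Gameplay Ability System.
; When a WorldDynamic or Pawn component enters its Box, the server applies both effect specs to every overlapping BP_AI, despite the asset's name.
; Each target's ability system component comes from its FirstLight player state.
; The Niagara effect's completion sets a short lifespan, while other hit and overlap events only print debug text.
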(event `self.ReceiveActorBeginOverlap`
  (params (OtherActor :type "Actor Object Reference"))
  (`KismetSystemLibrary.PrintString` "Overlap"))

(event `self.Niagara.OnSystemFinished`
  (params (PSystem :type "NiagaraComponent Object Reference"))
  (`self.SetLifeSpan` 1.0))

(event `self.Niagara.OnComponentHit`
  (params (HitComponent :type "PrimitiveComponent Object Reference") (OtherActor :type "Actor Object Reference") (OtherComp :type "PrimitiveComponent Object Reference") (NormalImpulse :type "Vector Structure") (Hit :type "HitResult Structure (by ref)"))
  (`/Engine/EditorBlueprintResources/StandardMacros.IsValid` OtherActor
    (:`Is Valid`
      (`KismetSystemLibrary.PrintString` "Comp Hit"))))

(event `self.Box.OnComponentBeginOverlap`
  (params (OverlappedComponent :type "PrimitiveComponent Object Reference") (OtherActor :type "Actor Object Reference") (OtherComp :type "PrimitiveComponent Object Reference") (OtherBodyIndex :type Integer) (bFromSweep :type Boolean) (SweepResult :type "HitResult Structure (by ref)"))
  (bind _returnvalue (`PrimitiveComponent.GetCollisionObjectType` OtherComp))
  (if (or (`|EnumEquality` _returnvalue "ECC_WorldDynamic") (`|EnumEquality` _returnvalue "ECC_Pawn"))
    (`/Engine/EditorBlueprintResources/ActorMacros.Switch Has Authority`
      (:`Authority`
        (for _array_element (`PrimitiveComponent.GetOverlappingActors` (`self.Box`) "/Game/FirstLight/AI/BP_AI.BP_AI_C")
          (bind _asfirst_light_character (cast `FirstLightCharacter` _array_element))
          (bind _returnvalue_2 (`AbilitySystemBlueprintLibrary.GetAbilitySystemComponent` (`FirstLightCharacter.GetFLPlayerState` _asfirst_light_character)))
          (`/Engine/EditorBlueprintResources/StandardMacros.IsValid` _returnvalue_2
            (:`Is Valid`
              (if true
                (`AbilitySystemComponent.BP_ApplyGameplayEffectSpecToSelf` _returnvalue_2 (`self.DamageEffectSpecHandle`))
                (`AbilitySystemComponent.BP_ApplyGameplayEffectSpecToSelf` _returnvalue_2 (`self.StunEffectSpecHandle`))))))))))

(fn `UserConstructionScript`)