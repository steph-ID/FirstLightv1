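; BP_ArenaGate is an arena gate that rises when the game starts.
; On BeginPlay it binds to the GameStart event of FirstLightArenaGameMode, which calls RaiseGate.
; The OpenGate timeline lerps Z between start and end heights, feeding world X and Y into a relative location setter.
; LowerGate reverses the timeline, though nothing in this Blueprint calls it.
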(event `RaiseGate`
  (bind (_returnvalue_x _returnvalue_y) (`KismetMathLibrary.BreakVector` (`self.K2_GetActorLocation`)))
  (bind (_direction _gateheight) (`Timeline|OpenGate` :!label _label)
    (:`Update`
      (`self.K2_SetActorRelativeLocation` (`KismetMathLibrary.MakeVector` _returnvalue_x _returnvalue_y (`KismetMathLibrary.Lerp` (`self.GateStartLocationZ`) (`self.GateEndLocationZ`) _gateheight))))))

(event `LowerGate`
  (goto _label :!via `Reverse`))

(event `self.ReceiveBeginPlay`
  (bind _asfirst_light_arena_game_mode (cast `FirstLightArenaGameMode` (`GameplayStatics.GetGameMode`)))
  (add `FirstLightArenaGameMode.GameStart` _asfirst_light_arena_game_mode (delegate `GameStart_Event`)))

(event `GameStart_Event`
  (`self.RaiseGate`))

(fn `UserConstructionScript`)