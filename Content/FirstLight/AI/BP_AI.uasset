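; Melee enemy character for an arena mode, with a health bar and a stealth-assassination victim routine behind a camera-facing proximity prompt.
; Damage triggers hit montages and knockback through BPCEnemyComponent; death ragdolls it, lowers the arena spawn count and awards XP and points.
; An index-driven montage combo supports buffered attacks, while timer-looped sphere traces between sword points damage tagged actors, with debug drawing left on.
; HandleDamage forwards a Weapon.Hit gameplay event to the instigator.
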(event `self.ReceiveBeginPlay`
  (bind _aswbp_enemy_health_bar (cast `/Game/FirstLight/UI/InWorldText/WBP_EnemyHealthBar` (`WidgetComponent.GetWidget` (`self.HealthBarWidget`))))
  (set `self.EnemyHealthBarUI` _aswbp_enemy_health_bar))

(event `HandleDamage`
  (params (Instigator :type "Controller Object Reference"))
  (`AbilitySystemBlueprintLibrary.SendGameplayEventToActor` Instigator (struct :`TagName` "Weapon.Hit") (make `GameplayEventData` (struct) Instigator self null null (struct) (struct) (struct) 0.0 (`AbilitySystemBlueprintLibrary.AbilityTargetDataFromActor` self))))

(event `self.ReceiveTick`
  (params (DeltaSeconds :type "Float (single-precision)"))
  (`SceneComponent.K2_SetWorldRotation` (`self.ExecuteWidget`) (`KismetMathLibrary.FindLookAtRotation` (`SceneComponent.K2_GetComponentLocation` (`self.ExecuteWidget`)) (`SceneComponent.K2_GetComponentLocation` (`PlayerCameraManager.TransformComponent` (`GameplayStatics.GetPlayerCameraManager` 0)))) false false)
  (`SceneComponent.K2_SetWorldRotation` (`self.HealthBarWidget`) (`KismetMathLibrary.FindLookAtRotation` (`SceneComponent.K2_GetComponentLocation` (`self.ExecuteWidget`)) (`SceneComponent.K2_GetComponentLocation` (`PlayerCameraManager.TransformComponent` (`GameplayStatics.GetPlayerCameraManager` 0)))) false false))

(event `self.ReceiveAnyDamage`
  (params (Damage :type "Float (single-precision)") (DamageType :type "DamageType Object Reference") (InstigatedBy :type "Controller Object Reference") (DamageCauser :type "Actor Object Reference"))
  (bind _charactermovement (`self.CharacterMovement`))
  (bind _damage_causer (`self.Damage Causer`))
  (bind _hitanims (`self.HitAnims`))
  (bind _bpc_enemycomponent (`self.BPC_EnemyComponent`))
  ;[0.05127 0.05127 0.05127] Take Damage
  (set `self.Damage Causer` DamageCauser)
  (`self.PlayAnimMontage` (`|GetArrayItem` _hitanims (`KismetMathLibrary.RandomIntegerInRange` 0 (- (`KismetArrayLibrary.Array_Length` _hitanims) 1))))
  (`|ExecutionSequence`
    (:`then_0`
      (`self.LaunchCharacter` (* (`KismetMathLibrary.GetForwardVector` (`self.K2_GetActorRotation` (select `bool` (`KismetSystemLibrary.IsValid` _damage_causer) :`false` self :`true` _damage_causer :!type "Actor Object Reference"))) 700.0))
      (`GameplayStatics.PlaySoundAtLocation` "/Game/FirstLight/Audio/Deaths/416839__tonsil5__grunt1-death-pain.416839__tonsil5__grunt1-death-pain" (`self.K2_GetActorLocation`) (struct) 1.0 (`KismetMathLibrary.RandomFloatInRange` 1.0 1.3) 0.0 null null null null))
    (:`then_1`
      (bind _isdead (`/Game/FirstLight/Blueprints/CharacterComponents/BPC_CharacterAttributes.DecreaseHealth` (`self.BPC_EnemyComponent`) Damage))
      (if _isdead
        (`CharacterMovementComponent.DisableMovement` _charactermovement)
        (`MovementComponent.StopMovementImmediately` _charactermovement)
        (`GameplayStatics.PlaySoundAtLocation` "/Game/FirstLight/Audio/Deaths/SC_M_Death.SC_M_Death" (`self.K2_GetActorLocation`) (struct) 1.0 1.0 0.0 null null null null)
        (`self.Ragdoll`)
        (`PrimitiveComponent.SetCollisionEnabled` (`self.CapsuleComponent`) "NoCollision")
        (`PrimitiveComponent.SetCollisionEnabled` (`self.ExecuteRadius`) "NoCollision")
        (bind _asbp_arena_game_state (cast `/Game/FirstLight/GameModes/BP_ArenaGameState` (`GameplayStatics.GetGameState`)))
        (`/Game/FirstLight/GameModes/BP_ArenaGameState.ReduceSpawnedCount` _asbp_arena_game_state)
        (bind _totalxp (`/Game/FirstLight/Blueprints/CharacterComponents/BPC_EnemyComponent.CalculateXpToGive` _bpc_enemycomponent))
        (bind _returnvalue (`/Game/FirstLight/Blueprints/CharacterComponents/BPC_EnemyComponent.CalculatePointsToGive` _bpc_enemycomponent))
        (bind _asbp_flchar (cast `/Game/FirstLight/Characters/BP_FLChar` (`self.Damage Causer`)))
        (bind _bpc_characterattributes (`/Game/FirstLight/Characters/BP_FLChar.BPC_CharacterAttributes` _asbp_flchar))
        (`/Game/FirstLight/Blueprints/CharacterComponents/BPC_CharacterAttributes.IncreaseXP` _bpc_characterattributes (`KismetMathLibrary.FTrunc` _totalxp))
        (`/Game/FirstLight/Blueprints/CharacterComponents/BPC_CharacterAttributes.IncreasePoints` _bpc_characterattributes _returnvalue)
        (`self.SetLifeSpan` 3.0)))))

(event `Ragdoll`
  ;[0.05127 0.05127 0.05127] Ragdoll
  (`PrimitiveComponent.SetSimulatePhysics` (`self.Mesh`) true))

(event `self.ExecuteRadius.OnComponentBeginOverlap`
  (params (OverlappedComponent :type "PrimitiveComponent Object Reference") (OtherActor :type "Actor Object Reference") (OtherComp :type "PrimitiveComponent Object Reference") (OtherBodyIndex :type Integer) (bFromSweep :type Boolean) (SweepResult :type "HitResult Structure (by ref)"))
  (cast `/Game/FirstLight/Characters/BP_CharacterBase` OtherActor)
  (`SceneComponent.SetVisibility` (`self.ExecuteWidget`) true false))

(event `self.ExecuteRadius.OnComponentEndOverlap`
  (params (OverlappedComponent :type "PrimitiveComponent Object Reference") (OtherActor :type "Actor Object Reference") (OtherComp :type "PrimitiveComponent Object Reference") (OtherBodyIndex :type Integer))
  (cast `/Game/FirstLight/Characters/BP_CharacterBase` OtherActor)
  (`SceneComponent.SetVisibility` (`self.ExecuteWidget`) false false))

(event `AIAttackCombo`
  ;[0.05127 0.05127 0.05127] Combo System
  ;;[0.05127 0.05127 0.05127] Attack Input
  (if (`self.CanAttack`)
    (`self.PrimaryAttack`)))

(event `Attack1`
  ;[0.05127 0.05127 0.05127] Combo System
  ;;[0.05127 0.05127 0.05127] Attack 1
  (`/Engine/EditorBlueprintResources/StandardMacros.DoOnce` false :!label _label
    (:`Completed`
      (`KismetSystemLibrary.Delay` 0.2)
      (`|PlayMontage` (`self.Mesh`) "/Game/FirstLight/Characters/Animations/Attacks/Sword/Attack1_Montage.Attack1_Montage"
        (:`then`
          (`/Engine/EditorBlueprintResources/StandardMacros.IncrementInt` (`self.AttackIndex`)
            (:`  `
              (goto _label :!via `Reset`))))))))

(event `PrimaryAttack`
  ;[0.05127 0.05127 0.05127] Combo System
  ;;[0.05127 0.05127 0.05127] Primary Attack
  (if (`self.IsAttacking`)
    (set `self.SaveAttack` true)
    (else
      (set `self.IsAttacking` true)
      (switch `int` (`self.AttackIndex`) :!label _label_2
        (:`0`
          (`self.Attack1`))
        (:`1`
          (`self.Attack2`))
        (:`2`
          (`self.Attack4`))))))

(event `Attack2`
  ;[0.05127 0.05127 0.05127] Combo System
  ;;[0.05127 0.05127 0.05127] Attack 2
  (`/Engine/EditorBlueprintResources/StandardMacros.DoOnce` false :!label _label_3
    (:`Completed`
      (`KismetSystemLibrary.Delay` 0.2)
      (`|PlayMontage` (`self.Mesh`) "/Game/FirstLight/Characters/Animations/Attacks/Sword/Attack2_Montage.Attack2_Montage"
        (:`then`
          (`/Engine/EditorBlueprintResources/StandardMacros.IncrementInt` (`self.AttackIndex`)
            (:`  `
              (goto _label_3 :!via `Reset`))))))))

(event `AttackCombo`
  ;[0.05127 0.05127 0.05127] Combo System
  ;;[0.05127 0.05127 0.05127] Continue Attack Combo
  (if (`self.SaveAttack`)
    (set `self.SaveAttack` false)
    (goto _label_2)
    (else
      (`self.StopCombo`))))

(event `Attack3`
  ;[0.05127 0.05127 0.05127] Combo System
  ;;[0.05127 0.05127 0.05127] Attack 3
  (`/Engine/EditorBlueprintResources/StandardMacros.DoOnce` false :!label _label_4
    (:`Completed`
      (`KismetSystemLibrary.Delay` 0.2)
      (`|PlayMontage` (`self.Mesh`) "/Game/FirstLight/Characters/Animations/Attacks/Sword/Kick_Montage.Kick_Montage"
        (:`then`
          (`/Engine/EditorBlueprintResources/StandardMacros.IncrementInt` (`self.AttackIndex`)
            (:`  `
              (goto _label_4 :!via `Reset`))))))))

(event `StopCombo`
  ;[0.05127 0.05127 0.05127] Combo System
  ;;[0.05127 0.05127 0.05127] Stop Attack/Combo
  (set `self.IsAttacking` false)
  (set `self.AttackIndex` 0))

(event `Attack4`
  ;[0.05127 0.05127 0.05127] Combo System
  ;;[0.05127 0.05127 0.05127] Attach 4
  (`/Engine/EditorBlueprintResources/StandardMacros.DoOnce` false :!label _label_5
    (:`Completed`
      (`KismetSystemLibrary.Delay` 0.2)
      (`|PlayMontage` (`self.Mesh`) "/Game/FirstLight/Characters/Animations/Attacks/Sword/Attack3_Montage.Attack3_Montage"
        (:`then`
          (`/Engine/EditorBlueprintResources/StandardMacros.IncrementInt` (`self.AttackIndex`)
            (:`  `
              (goto _label_5 :!via `Reset`))))))))

(event `StartSwordTrace`
  ;[0.05127 0.05127 0.05127] Sword Trace
  (bind _returnvalue (`KismetSystemLibrary.K2_SetTimerDelegate` (delegate `SwordTraceLoop`) 0.001 true))
  (set `self.SwordTraceLoopTimer` _returnvalue))

(event `SphereTrace`
  ;[0.05127 0.05127 0.05127] Sphere Trace (Stab & Kick)
)

(event `SwordTraceLoop`
  ;[0.05127 0.05127 0.05127] Sword Trace
  (bind (_outhit _returnvalue) (`KismetSystemLibrary.SphereTraceSingle` :`Start` (`SceneComponent.K2_GetComponentLocation` (`self.SwordTopPoint`)) :`End` (`SceneComponent.K2_GetComponentLocation` (`self.SwordBottomPoint`)) :`Radius` 15.0 :`TraceChannel` "TraceTypeQuery1" :`DrawDebugType` "ForDuration" :`DrawTime` (`self.DrawTime`)))
  (if _returnvalue
    (bind (_bblockinghit _binitialoverlap _time _distance _location _impactpoint _normal _impactnormal _physmat _hitactor) (`GameplayStatics.BreakHitResult` _outhit))
    (`/Engine/EditorBlueprintResources/StandardMacros.IsValid` _hitactor
      (:`Is Valid`
        (if (`self.ActorHasTag` _hitactor "DamageableByAI")
          (`/Engine/EditorBlueprintResources/StandardMacros.DoOnce` false :!label _label_6
            (:`Completed`
              (bind _returnvalue_2 (`GameplayStatics.ApplyDamage` _hitactor 10.0 null self))
              (`GameplayStatics.SpawnEmitterAtLocation` "/Game/Realistic_Starter_VFX_Pack_Vol2/Particles/Blood/P_Blood_Splat_Cone.P_Blood_Splat_Cone" _location (`KismetMathLibrary.MakeRotFromXY` _normal _normal) (0.4 0.4 0.4) true "AutoRelease")
              (`KismetSystemLibrary.Delay` 0.5)
              (goto _label_6 :!via `Reset`))))))))

(event `StopSwordTrace`
  ;[0.05127 0.05127 0.05127] Sword Trace
  (`KismetSystemLibrary.K2_ClearAndInvalidateTimerHandle` (`self.SwordTraceLoopTimer`)))

(event `PlaySwordHitSounds`
  ;[0.05127 0.05127 0.05127] Sword Hit Sounds
  (`GameplayStatics.PlaySoundAtLocation` "/Game/FirstLight/Audio/SwordHits/MS_SwordHit.MS_SwordHit" (`self.K2_GetActorLocation` (`self.GetOwner`)) (struct) 1.0 1.0 0.0 null null null null))

(fn `Attack`
  (returns (AnimationDuration :type "Float (double-precision)"))
  (`self.AIAttackCombo`)
  (return 0.0))

(fn `DisplayDamageToActor`
  (params (DamageDone :type Integer))
  (bind _returnvalue (`|CreateWidget` "/Game/FirstLight/UI/InWorldText/WBP_CombatDamage.WBP_CombatDamage_C"))
  (`TextBlock.SetText` (`/Game/FirstLight/UI/InWorldText/WBP_CombatDamage.CombatDamage_Text` _returnvalue) (`KismetTextLibrary.Conv_IntToText` DamageDone)))

(fn `PlayWeaponHitSound`
  (`GameplayStatics.PlaySoundAtLocation` "/Game/FirstLight/Audio/SwordHits/MS_SwordHit.MS_SwordHit" (`self.K2_GetActorLocation` (`self.GetOwner`)) (struct) 1.0 1.0 0.0 null null null null))

(fn `StealthBackAssassin`
  (returns (ReferenceLocation :type "Vector Structure") (KillRotation :type "Rotator Structure"))
  (`self.PlayAnimMontage` "/Game/FirstLight/Characters/Animations/Attacks/Paired_Knife_Stealth_KidneyAndNeck_Vic_Montage.Paired_Knife_Stealth_KidneyAndNeck_Vic_Montage")
  (`self.Ragdoll`)
  (`SceneComponent.SetVisibility` (`self.ExecuteWidget`) false false)
  (return (`SceneComponent.K2_GetComponentLocation` (`self.KillReference`)) (`self.K2_GetActorRotation`)))

(fn `UserConstructionScript`)