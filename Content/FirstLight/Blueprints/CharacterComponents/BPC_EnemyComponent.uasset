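; BPC_EnemyComponent is the enemy character component that sets up NPC data and health bar UI and calculates kill rewards.
; Attributes come from a data table row or SetEnemy, then next-tick initialization caches the BP_AI owner and fills health, level and name.
; DecreaseHealth decrements the arena's EnemiesAlive when the parent call returns true.
; Points scale by enemy type, while XP returns unscaled BaseXP, leaving the level-curve formula unused.
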(event `self.ReceiveBeginPlay`)

(event `InitializeNPCData`
  (bind _enemyhealthbarui (`/Game/FirstLight/AI/BP_AI.EnemyHealthBarUI` (`self.AICharacter`)))
  (`KismetSystemLibrary.DelayUntilNextTick`)
  (`|ExecutionSequence`
    (:`then_0`
      (bind _asbp_ai (cast `/Game/FirstLight/AI/BP_AI` (`self.GetOwner`)))
      (set `self.AICharacter` _asbp_ai)
      (set `self.CharacterMesh` (`Character.Mesh` _asbp_ai))
      (set `self.IsPlayer` false))
    (:`then_1`
      (set `self.HealthBar` (`/Game/FirstLight/UI/InWorldText/WBP_EnemyHealthBar.HealthBar` _enemyhealthbarui))
      (set `self.HealthBarText` (`/Game/FirstLight/UI/InWorldText/WBP_EnemyHealthBar.EnemyHealth_TextBlock` _enemyhealthbarui))
      (set `self.LevelTextObj` (`/Game/FirstLight/UI/InWorldText/WBP_EnemyHealthBar.EnemyLevel_TextBlock` _enemyhealthbarui))
      (set `self.EnemyNameTextBlock` (`/Game/FirstLight/UI/InWorldText/WBP_EnemyHealthBar.EnemyName_TextBlock` _enemyhealthbarui)))
    (:`then_2`
      (`self.SetHealthBar`)
      (`self.SetLevelText`)
      (`self.SetCharacterName` (`/Game/FirstLight/UI/InWorldText/WBP_EnemyHealthBar.EnemyName_TextBlock` (`/Game/FirstLight/AI/BP_AI.EnemyHealthBarUI` (`self.AICharacter`)))))))

(fn `CalculatePointsToGive`
  (returns (ReturnValue :type Integer))
  (bind (_npcattributes_name _npcattributes_level _npcattributes_type) (break `/Game/FirstLight/Data/Character/Enemy/S_EnemyData` (`self.NpcAttributes`)))
  (bind _returnvalue (* (select `/Game/FirstLight/Data/Character/Enemy/E_EnemyTypes` _npcattributes_type :`NewEnumerator0` 1 :`NewEnumerator2` 2 :`NewEnumerator1` 3 :`NewEnumerator3` 4 :!type "Byte") 5))
  (`KismetSystemLibrary.PrintString` (`KismetStringLibrary.Conv_ByteToString` _returnvalue))
  (return (`KismetMathLibrary.Conv_ByteToInt` _returnvalue)))

(fn `CalculateXpToGive`
  (returns (TotalXP :type "Float (double-precision)"))
  (bind (_npcattributes_name _npcattributes_level _npcattributes_type _npcattributes_element _npcattributes_basexp) (break `/Game/FirstLight/Data/Character/Enemy/S_EnemyData` (`self.NpcAttributes`)))
  (bind _returnvalue (`|GetDataTableRow` (break `DataTableRowHandle` (break `/Game/FirstLight/Data/Common/S_DataTableRow` (`self.StatMultipliers`))) (`KismetStringLibrary.Conv_StringToName` (`|GetEnumeratorNameAsString` _npcattributes_type)))
    (:`then`
      (return (`KismetMathLibrary.Conv_IntToDouble` _npcattributes_basexp)))))

(fn `DecreaseHealth`
  (params (Damage :type "Float (double-precision)"))
  (returns (IsDead :type Boolean))
  (bind _isdead (`parent.DecreaseHealth` Damage))
  (if _isdead
    (bind _asbp_arena_game_state (cast `/Game/FirstLight/GameModes/BP_ArenaGameState` (`GameplayStatics.GetGameState`)))
    (`/Engine/EditorBlueprintResources/StandardMacros.DecrementInt` (`/Game/FirstLight/GameModes/BP_ArenaGameState.EnemiesAlive` _asbp_arena_game_state)
      (:`  `
        (return _isdead)))))

(fn `InitializeNPC`
  (params (NpcData :type "/Game/FirstLight/Data/Common/S_DataTableRow Structure"))
  (bind _output_get (set `self.NpcDataEC` NpcData))
  (bind _returnvalue (`|GetDataTableRow` (break `DataTableRowHandle` (break `/Game/FirstLight/Data/Common/S_DataTableRow` _output_get)) (`.RowName` (break `DataTableRowHandle` (break `/Game/FirstLight/Data/Common/S_DataTableRow` _output_get))))
    (:`then`
      (set `self.NpcAttributes` _returnvalue)
      (`self.InitializeNPCData`))))

(fn `SetEnemy`
  (params (NpcAttributes :type "/Game/FirstLight/Data/Character/Enemy/S_EnemyData Structure"))
  (bind _output_get (set `self.NpcAttributes` NpcAttributes))
  (set `self.CharacterName` (break `/Game/FirstLight/Data/Character/Enemy/S_EnemyData` _output_get))
  (`self.InitializeNPCData`))