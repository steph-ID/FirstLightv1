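; BP_GA_AutoAttack is a Gameplay Ability that starts the player character's primary auto attack.
; Activation resolves the character through the owning PlayerState, flags its BPAttackSystem as attacking and calls PrimaryAttack when CanAttack allows.
; Ending the ability clears that flag.
; The Weapon.Hit event wait that applies GE_Damage and ends the ability is disconnected, so the live graph neither applies damage nor ends itself.
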(event `self.K2_ActivateAbility`
  (bind _asbp_player_state (cast `/Game/FirstLight/GameModes/BP_PlayerState` (`self.GetOwningActorFromActorInfo`)))
  (bind _asbp_flchar (cast `/Game/FirstLight/Characters/BP_FLChar` (`PlayerState.GetPawn` _asbp_player_state)))
  (bind _bp_attacksystem (`/Game/FirstLight/Characters/BP_FLChar.BP_AttackSystem` _asbp_flchar))
  (set `/Game/FirstLight/Blueprints/CharacterComponents/BP_AttackSystem.IsAttacking` true _bp_attacksystem)
  (if (`/Game/FirstLight/Blueprints/CharacterComponents/BP_AttackSystem.CanAttack` _bp_attacksystem)
    (`/Game/FirstLight/Blueprints/CharacterComponents/BP_AttackSystem.PrimaryAttack` _bp_attacksystem)))

(event `self.K2_OnEndAbility`
  (params (bWasCancelled :type Boolean))
  (bind _weaponhittask (`self.WeaponHitTask`))
  (set `/Game/FirstLight/Blueprints/CharacterComponents/BP_AttackSystem.IsAttacking` false (`/Game/FirstLight/Characters/BP_FLChar.BP_AttackSystem` (stale `self.K2_ActivateAbility` _asbp_flchar)))
  (`/Engine/EditorBlueprintResources/StandardMacros.IsValid` _weaponhittask
    (:`Is Valid`
      (`GameplayTask.EndTask` _weaponhittask))))