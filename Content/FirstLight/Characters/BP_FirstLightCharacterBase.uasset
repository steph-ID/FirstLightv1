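; Base character Blueprint for First Light that handles spawned NPC setup, damage reactions and death.
; Setup functions copy spawn info into identity fields and an attribute map, and apply a single skeletal mesh.
; Damage triggers knockback, a pitch-varied grunt and camera shake, then lowers health through BPCCharacterAttributes.
; Death disables collision and movement, reduces the arena's spawn count, and awards a BP_FLChar killer XP and points before timed removal.
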(event `self.ReceiveBeginPlay`)

(event `self.ReceiveAnyDamage`
  (params (Damage :type "Float (single-precision)") (DamageType :type "DamageType Object Reference") (InstigatedBy :type "Controller Object Reference") (DamageCauser :type "Actor Object Reference"))
  (bind _returnvalue (`self.K2_GetActorLocation`))
  ;[0.05127 0.05127 0.05127] Apply Damage
  (`|ExecutionSequence`
    (:`then_0`
      (`/Engine/EditorBlueprintResources/StandardMacros.IsValid` DamageCauser
        (:`Is Valid`
          (`self.LaunchCharacter` (* (`KismetMathLibrary.GetForwardVector` (`self.K2_GetActorRotation` DamageCauser)) 300.0)))
        (:`Is Not Valid`
          _))
      (`GameplayStatics.PlaySoundAtLocation` "/Game/FirstLight/Audio/Deaths/416839__tonsil5__grunt1-death-pain.416839__tonsil5__grunt1-death-pain" _returnvalue (struct) 1.0 (`KismetMathLibrary.RandomFloatInRange` 1.0 1.3) 0.0 null null null null)
      (`GameplayStatics.PlayWorldCameraShake` "/Game/FirstLight/Blueprints/BP_SwordHitCameraShake.BP_SwordHitCameraShake_C" _returnvalue 0.0 2000.0))
    (:`then_1`
      (bind _isdead (`/Game/FirstLight/Blueprints/CharacterComponents/BPC_CharacterAttributes.DecreaseHealth` (`self.BPC_CharacterAttributes`) Damage))
      (bind _output_get (set `self.IsDead` _isdead))
      (if _output_get
        (`self.ProcessNPCDeath` DamageCauser)))))

(fn `ProcessNPCDeath`
  (params (`Damage Causer` :type "Actor Object Reference"))
  (bind _bpc_npccomponent (`self.BPC_NPCComponent`))
  (bind _charactermovement (`self.CharacterMovement`))
  (if (`self.IsDead`)
    (`|ExecutionSequence`
      (:`then_0`
        (`PrimitiveComponent.SetCollisionEnabled` (`self.CapsuleComponent`) "NoCollision")
        (`PrimitiveComponent.SetCollisionEnabled` (`self.Mesh`) "NoCollision")
        (`PrimitiveComponent.SetCollisionEnabled` (`self.EnemyCollision`) "NoCollision")
        (`CharacterMovementComponent.DisableMovement` _charactermovement)
        (`MovementComponent.StopMovementImmediately` _charactermovement))
      (:`then_1`
        (bind _asbp_arena_game_state (cast `/Game/FirstLight/GameModes/BP_ArenaGameState` (`GameplayStatics.GetGameState`)))
        (`/Game/FirstLight/GameModes/BP_ArenaGameState.ReduceSpawnedCount` _asbp_arena_game_state))
      (:`then_2`
        (bind _totalxp (`/Game/FirstLight/Blueprints/CharacterComponents/BPC_NPCComponent.CalculateXpToGive` _bpc_npccomponent))
        (bind _returnvalue (`/Game/FirstLight/Blueprints/CharacterComponents/BPC_NPCComponent.CalculatePointsToGive` _bpc_npccomponent))
        (bind _asbp_flchar (cast `/Game/FirstLight/Characters/BP_FLChar` `Damage Causer`))
        (bind _bpc_characterattributes (`/Game/FirstLight/Characters/BP_FLChar.BPC_CharacterAttributes` _asbp_flchar))
        (`/Game/FirstLight/Blueprints/CharacterComponents/BPC_CharacterAttributes.IncreaseXP` _bpc_characterattributes (`KismetMathLibrary.FTrunc` _totalxp))
        (`/Game/FirstLight/Blueprints/CharacterComponents/BPC_CharacterAttributes.IncreasePoints` _bpc_characterattributes _returnvalue)
        (`self.SetLifeSpan` 3.0)))))

(fn `SetNPCCharacterBP`
  (params (SkeletalMesh :type "Array of SkeletalMesh Object Reference") (MaterialInstances :type "Array of SkeletalMesh Object Reference") (AnimationBP :type "AnimInstance Object Reference"))
  (`|ExecutionSequence`
    (:`then_0`
      (for _array_element SkeletalMesh
        (if (== (`KismetArrayLibrary.Array_Length` SkeletalMesh) 1)
          (`SkeletalMeshComponent.SetSkeletalMeshAsset` (`self.Mesh`) _array_element)
          (`SkeletalMeshComponent.SetAnimInstanceClass` (`self.Mesh`) null))))))

(fn `SetNPCCharacterModel`
  (params (SkeletalMesh :type "Array of SkeletalMesh Object Reference") (MaterialInstances :type "Array of SkeletalMesh Object Reference") (AnimationBP :type "AnimInstance Object Reference") (CharacterBP :type "FirstLightCharacterBase Class Reference"))
  (`|ExecutionSequence`
    (:`then_0`
      (for _array_element SkeletalMesh
        (if (== (`KismetArrayLibrary.Array_Length` SkeletalMesh) 1)
          (`SkeletalMeshComponent.SetSkeletalMeshAsset` (`self.Mesh`) _array_element)
          (`SkeletalMeshComponent.SetAnimInstanceClass` (`self.Mesh`) null))))))

(fn `SetNPCData`
  (params (SpawnedNPCInfo :type "/Game/FirstLight/Data/Character/Enemy/S_EnemyData Structure"))
  (bind _output_get (set `self.SpawnedNPCInfo` SpawnedNPCInfo))
  (`|ExecutionSequence`
    (:`then_0`
      (set `self.NPCName` (break `/Game/FirstLight/Data/Character/Enemy/S_EnemyData` _output_get))
      (set `self.NPCLevel` (`.Level_4_17DDD007429A5D93A0361D8776C91288` (break `/Game/FirstLight/Data/Character/Enemy/S_EnemyData` _output_get)))
      (set `self.NPCRarityType` (`.Type_10_BBB0DA1F467BFE6397D6F0B4CB365E6D` (break `/Game/FirstLight/Data/Character/Enemy/S_EnemyData` _output_get)))
      (set `self.NPCElement` (`.Element_7_22DA82D848580121E08E75AC8068C5A6` (break `/Game/FirstLight/Data/Character/Enemy/S_EnemyData` _output_get))))
    (:`then_1`
      (for _array_element (`.Attributes_28_0E61342B4D1278B17FC275A5E5E133AB` (break `/Game/FirstLight/Data/Character/Enemy/S_EnemyData` _output_get))
        (`BlueprintMapLibrary.Map_Add` (`self.CharacterStattributeData`) (break `/Game/FirstLight/Data/Common/S_AttributeForDatatables` _array_element) (make `/Game/FirstLight/Data/Character/S_CharAttribute` (break `/Game/FirstLight/Data/Common/S_AttributeForDatatables` _array_element) (`.AttributeValue_5_FC06B5EB459EDC595E33EEB9F677AEA0` (break `/Game/FirstLight/Data/Common/S_AttributeForDatatables` _array_element))))))))

(fn `UserConstructionScript`)