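; Arena enemy spawner that spawns a batch of BP_AI_Enemy whenever the BP_ArenaGameState spawn event fires.
; The construction script sorts enemy data table rows into Common, Elite, Rare and Boss pools.
; Each enemy spawns at a random X/Y offset and gets a random row from EnemyTypeToSpawn, Elite or Rare through its enemy component.
; The batch grows by one per call until it equals MaxEnemyCount.
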(event `self.ReceiveBeginPlay`
  (bind _asbp_arena_game_state (cast `/Game/FirstLight/GameModes/BP_ArenaGameState` (`GameplayStatics.GetGameState`)))
  (add `/Game/FirstLight/GameModes/BP_ArenaGameState.SpawnEnemy` _asbp_arena_game_state (delegate `SpawnEnemy`)))

(event `SpawnEnemy`
  (bind _returnvalue (`self.GetTransform`))
  (for _ (range (`self.EnemiesToSpawn`))
    (bind _returnvalue_2 (`|SpawnActorFromClass` "/Game/FirstLight/AI/Test/BP_AI_Enemy.BP_AI_Enemy_C" (`KismetMathLibrary.MakeTransform` (`KismetMathLibrary.MakeVector` (+ (.x (.location _returnvalue)) (`KismetMathLibrary.RandomFloatInRange` (`self.MinRange`) (`self.MaxRange`))) (+ (.y (.location _returnvalue)) (`KismetMathLibrary.RandomFloatInRange` (`self.MinRange`) (`self.MaxRange`))) (.z (.location _returnvalue))) (.rotation _returnvalue)) "AdjustIfPossibleButAlwaysSpawn" "OverrideRootScale" null null))
    (bind _randomenemy (`self.GetRandomEnemy` (select `int` (`KismetMathLibrary.RandomIntegerInRange` 0 2) :`0` (`self.EnemyTypeToSpawn`) :`1` "NewEnumerator2" :`2` "NewEnumerator1")))
    (`/Game/FirstLight/Blueprints/CharacterComponents/BPC_EnemyComponent.SetEnemy` (`/Game/FirstLight/AI/Test/BP_AI.BPC_EnemyComponent` _returnvalue_2) _randomenemy))
  (if (not (== (`self.MaxEnemyCount`) (`self.EnemiesToSpawn`)))
    (`/Engine/EditorBlueprintResources/StandardMacros.IncrementInt` (`self.EnemiesToSpawn`))))

(event `CountWaves`
  (params (EnemiesToSpawn :type Integer)))

(fn `GetRandomEnemy`
  (params (EnemyTypeToSpawn :type "/Game/FirstLight/Data/Character/Enemy/E_EnemyTypes Enum" :default "NewEnumerator0"))
  (returns (RandomEnemy :type "/Game/FirstLight/Data/Character/Enemy/S_EnemyData Structure (by ref)"))
  (bind _returnvalue (select `/Game/FirstLight/Data/Character/Enemy/E_EnemyTypes` EnemyTypeToSpawn :`NewEnumerator0` (`self.CommonEnemies`) :`NewEnumerator2` (`self.EliteEnemies`) :`NewEnumerator1` (`self.RareEnemies`) :`NewEnumerator3` (`self.BossEnemies`)))
  (return (`|GetArrayItem` _returnvalue (`KismetMathLibrary.RandomIntegerInRange` 0 (- (`KismetArrayLibrary.Array_Length` _returnvalue) 1)))))

(fn `SetSpawnableEnemies`
  (bind _outrownames (`DataTableFunctionLibrary.GetDataTableRowNames` "/Game/FirstLight/Data/Character/Enemy/DT_Enemies.DT_Enemies"))
  (for _array_element _outrownames
    (bind _returnvalue (`|GetDataTableRow` (`self.EnemyTable`) _array_element)
      (:`then`
        (switch `/Game/FirstLight/Data/Character/Enemy/E_EnemyTypes` (`.Type_10_BBB0DA1F467BFE6397D6F0B4CB365E6D` (break `/Game/FirstLight/Data/Character/Enemy/S_EnemyData` _returnvalue))
          (:`NewEnumerator0`
            (`KismetArrayLibrary.Array_Add` (`self.CommonEnemies`) _returnvalue))
          (:`NewEnumerator2`
            (`KismetArrayLibrary.Array_Add` (`self.EliteEnemies`) _returnvalue))
          (:`NewEnumerator1`
            (`KismetArrayLibrary.Array_Add` (`self.RareEnemies`) _returnvalue))
          (:`NewEnumerator3`
            (`KismetArrayLibrary.Array_Add` (`self.BossEnemies`) _returnvalue)))))))

(fn `UserConstructionScript`
  (`self.SetSpawnableEnemies`))