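; NPC component for enemy characters that holds their identity and stats, drives their health bar widget and computes kill rewards.
; InitializeNPC reads attributes from a data table, while SetNPC applies supplied ones, fills the stat map and tags damageable owners.
; Both rebuild the widget's health, level and name display.
; XP returns unscaled BaseXP, with level-curve scaling left unwired, while points scale by rarity.
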(event `self.ReceiveBeginPlay`
  (bind _asbp_ai_enemy_npcbase (cast `/Game/FirstLight/AI/BP_AI_EnemyNPCBase` (`self.GetOwner`)))
  (bind _output_get (set `self.EnemyNPCCharacter` _asbp_ai_enemy_npcbase))
  (set `self.CharacterMesh` (`Character.Mesh` _asbp_ai_enemy_npcbase))
  (`KismetSystemLibrary.DelayUntilNextTick`)
  (`/Game/FirstLight/AI/BP_AI_EnemyNPCBase.InitializeEnemyWidget` _output_get)
  (set `self.IsPlayer` false))

(event `BuildNPCDataWidget`
  (`KismetSystemLibrary.DelayUntilNextTick`)
  (`|ExecutionSequence`
    (:`then_0`
      (bind _aswbp_enemy_health_bar (cast `/Game/FirstLight/Blueprints/UI/InWorldText/WBP_EnemyHealthBar` (`WidgetComponent.GetWidget` (`/Game/FirstLight/AI/BP_AI_EnemyNPCBase.HealthBarWidget` (`self.EnemyNPCCharacter`)))))
      (bind _output_get (set `self.HealthBar` (`/Game/FirstLight/Blueprints/UI/InWorldText/WBP_EnemyHealthBar.HealthBar` _aswbp_enemy_health_bar)))
      (`self.SetHealthBar` _output_get (`/Game/FirstLight/Blueprints/UI/InWorldText/WBP_EnemyHealthBar.EnemyHealth_TextBlock` _aswbp_enemy_health_bar))
      (`self.SetLevelText` (`/Game/FirstLight/Blueprints/UI/InWorldText/WBP_EnemyHealthBar.EnemyLevel_TextBlock` _aswbp_enemy_health_bar))
      (`self.SetCharacterName` (`/Game/FirstLight/Blueprints/UI/InWorldText/WBP_EnemyHealthBar.EnemyName_TextBlock` _aswbp_enemy_health_bar)))))

(fn `CalculatePointsToGive`
  (returns (ReturnValue :type Integer))
  (bind (_npcattributes_name _npcattributes_level _npcattributes_basexp _npcattributes_type) (break `/Game/FirstLight/Data/Character/Enemy/S_EnemyData` (`self.NpcAttributes`)))
  (return (`KismetMathLibrary.Conv_ByteToInt` (* (select `/Game/FirstLight/Data/Character/Enemy/E_EnemyTypes` _npcattributes_type :`NewEnumerator0` 1 :`NewEnumerator2` 2 :`NewEnumerator1` 3 :`NewEnumerator3` 4 :!type "Byte") 5))))

(fn `CalculateXpToGive`
  (returns (TotalXP :type "Float (double-precision)"))
  (bind (_npcattributes_name _npcattributes_level _npcattributes_basexp _npcattributes_type) (break `/Game/FirstLight/Data/Character/Enemy/S_EnemyData` (`self.NpcAttributes`)))
  (bind _returnvalue (`|GetDataTableRow` (break `DataTableRowHandle` (break `/Game/FirstLight/Data/Common/S_DataTableRow` (`self.StatMultipliers`))) (`KismetStringLibrary.Conv_StringToName` (`|GetEnumeratorNameAsString` _npcattributes_type)))
    (:`then`
      (return (`KismetMathLibrary.Conv_IntToDouble` _npcattributes_basexp)))))

(fn `DecreaseHealth`
  (params (Damage :type "Float (double-precision)"))
  (returns (IsDead :type Boolean))
  (bind _isdead (`parent.DecreaseHealth` Damage))
  (if _isdead
    (return _isdead)))

(fn `InitializeNPC`
  (params (NpcData :type "/Game/FirstLight/Data/Common/S_DataTableRow Structure"))
  (bind _output_get (set `self.NpcDataEC` NpcData))
  (bind _returnvalue (`|GetDataTableRow` (break `DataTableRowHandle` (break `/Game/FirstLight/Data/Common/S_DataTableRow` _output_get)) (`.RowName` (break `DataTableRowHandle` (break `/Game/FirstLight/Data/Common/S_DataTableRow` _output_get))))
    (:`then`
      (set `self.NpcAttributes` _returnvalue)
      (`self.BuildNPCDataWidget`))))

(fn `SetNPC`
  (params (NpcAttributes :type "/Game/FirstLight/Data/Character/Enemy/S_EnemyData Structure"))
  (bind _output_get (set `self.NpcAttributes` NpcAttributes))
  (`|ExecutionSequence`
    (:`then_0`
      (set `self.CharacterName` (break `/Game/FirstLight/Data/Character/Enemy/S_EnemyData` _output_get))
      (set `self.NPCLevel` (`.Level_4_17DDD007429A5D93A0361D8776C91288` (break `/Game/FirstLight/Data/Character/Enemy/S_EnemyData` _output_get)))
      (set `self.NPCRarityType` (`.Type_10_BBB0DA1F467BFE6397D6F0B4CB365E6D` (break `/Game/FirstLight/Data/Character/Enemy/S_EnemyData` _output_get)))
      (set `self.NPCElement` (`.Element_7_22DA82D848580121E08E75AC8068C5A6` (break `/Game/FirstLight/Data/Character/Enemy/S_EnemyData` _output_get)))
      (bind _asbp_first_light_character_base (cast `/Game/FirstLight/Characters/BP_FirstLightCharacterBase` (`self.GetOwner`)))
      (if (`.IsDamageable_50_7F4C451C4E16C214CA9679A2B8364D22` (break `/Game/FirstLight/Data/Character/Enemy/S_EnemyData` _output_get))
        (`KismetArrayLibrary.Array_Add` (`Actor.Tags` _asbp_first_light_character_base) "Damageable")))
    (:`then_1`
      (`self.BuildNPCDataWidget`))
    (:`then_2`
      (for _array_element (`.Attributes_28_0E61342B4D1278B17FC275A5E5E133AB` (break `/Game/FirstLight/Data/Character/Enemy/S_EnemyData` _output_get))
        (`BlueprintMapLibrary.Map_Add` (`self.CharacterStattributeData`) (break `/Game/FirstLight/Data/Common/S_AttributeForDatatables` _array_element) (make `/Game/FirstLight/Data/Character/S_CharAttribute` (break `/Game/FirstLight/Data/Common/S_AttributeForDatatables` _array_element) (`.AttributeValue_5_FC06B5EB459EDC595E33EEB9F677AEA0` (break `/Game/FirstLight/Data/Common/S_AttributeForDatatables` _array_element))))))))