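; Equipment component for BP_FLChar that handles weapon pickup and toggles the equipment menu.
; Interact sphere-traces from the follow camera, storing hit weapons in WeaponSlots and destroying the pickup, except animated weapons on arena maps, which equip through the character and stay in the world.
; The menu input creates or removes WBP_Equipment, switching attack permission, cursor, input mode and movement.
; A debug key prints the stored weapons.
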(event Input|EnhancedActionEvents|EnhancedInputActionIA_Interact
  (params (ActionValue :type Boolean) (ElapsedSeconds :type Float%20%28double-precision%29) (TriggeredSeconds :type Float%20%28double-precision%29) (InputAction :type Input%20Action%20Object%20Reference :default "/Game/FirstLight/Characters/Input/Actions/IA_Interact.IA_Interact"))
  (bind _characterref (Variables|Default|GetCharacterRef))
  (bind _followcamera (Variables|/Script/FirstLight.FirstLightPlayerCharacter|GetFollowCamera _characterref))
  (bind _returnvalue (Transformation|GetWorldLocation _followcamera))
  ;[0.05127 0.05127 0.05127] Pickup Trace
  (:Started
    (bind (_outhit _returnvalue_2) (Collision|SphereTraceForObjects _returnvalue (+ _returnvalue (* (Math|Vector|GetForwardVector (Transformation|GetWorldRotation _followcamera)) 1e+03)) 5e+01 (Utilities|Array|MakeArray "ObjectTypeQuery2") false 0 "ForDuration"))
    (if _returnvalue_2
      (bind _asbp_weapon (Utilities|Casting|CastToBP_Weapon (.HitActor (Collision|BreakHitResult _outhit)))
        (:then
          (CallFunction|AddWeapontoInventory (Variables|/Game/FirstLight/Data/Weapons/BP_Weapon.BP_Weapon_C|GetItemData _asbp_weapon))
          (Actor|DestroyActor _asbp_weapon)
          (Development|PrintString "Item collected"))
        (:CastFailed
          (bind _asbp_animated_weapon (Utilities|Casting|CastToBP_AnimatedWeapon (.HitActor (Collision|BreakHitResult _outhit))))
          (bind _asbp_arena_game_state (Utilities|Casting|CastToBP_ArenaGameState (Game|GetGameState)))
          (if (Variables|/Game/FirstLight/GameModes/BP_ArenaGameState.BP_ArenaGameState_C|GetArenaMap _asbp_arena_game_state)
            (CallFunction|EquipWeapon (Variables|/Game/FirstLight/Data/Weapons/BP_AnimatedWeapon.BP_AnimatedWeapon_C|GetItemData _asbp_animated_weapon))
            (else
              (CallFunction|AddWeapontoInventory (Variables|/Game/FirstLight/Data/Weapons/BP_AnimatedWeapon.BP_AnimatedWeapon_C|GetItemData _asbp_animated_weapon))
              (Actor|DestroyActor _asbp_animated_weapon))))))))

(event Input|EnhancedActionEvents|EnhancedInputActionIA_EquipmentMenu
  (params (ActionValue :type Boolean) (ElapsedSeconds :type Float%20%28double-precision%29) (TriggeredSeconds :type Float%20%28double-precision%29) (InputAction :type Input%20Action%20Object%20Reference :default "/Game/FirstLight/Characters/Input/Actions/IA_EquipmentMenu.IA_EquipmentMenu"))
  (bind _returnvalue (Game|GetPlayerController 0))
  (bind _characterref (Variables|Default|GetCharacterRef))
  (bind _attacksystem (Variables|Default|GetAttackSystem))
  ;[0.05127 0.05127 0.05127] Equipment Menu Panel
  (:Started
    (if (not (Variables|Default|GetIsPanelOpen))
      (Variables|/Game/FirstLight/Blueprints/CharacterComponents/BP_AttackSystem.BP_AttackSystem_C|SetCanAttack _attacksystem false)
      (bind _returnvalue_2 (UserInterface|CreateWidget "/Game/FirstLight/Systems/Equipment/UI/WBP_Equipment.WBP_Equipment_C" (Game|GetPlayerController 0)))
      (bind _output_get (Variables|Default|SetEquipmentWidget _returnvalue_2))
      (UserInterface|Viewport|AddtoViewport _output_get 0)
      (Variables|Default|SetIsPanelOpen true)
      (Variables|/Script/Engine.PlayerController|SetbShowMouseCursor _returnvalue true)
      (Input|SetInputModeGameandUI _returnvalue (Variables|Default|GetEquipmentWidget) "DoNotLock" false false)
      (Pawn|Components|CharacterMovement|SetMovementMode (Variables|/Script/Engine.Character|GetCharacterMovement _characterref) "MOVE_None" 0)
      (else
        (Variables|/Game/FirstLight/Blueprints/CharacterComponents/BP_AttackSystem.BP_AttackSystem_C|SetCanAttack _attacksystem true)
        (bind _equipmentwidget (Variables|Default|GetEquipmentWidget)
          (:then
            (Widget|RemovefromParent _equipmentwidget)
            (Variables|Default|SetEquipmentWidget 0)
            (Variables|Default|SetIsPanelOpen false)
            (Variables|/Script/Engine.PlayerController|SetbShowMouseCursor _returnvalue false)
            (Input|SetInputModeGameOnly _returnvalue false)
            (Pawn|Components|CharacterMovement|SetMovementMode (Variables|/Script/Engine.Character|GetCharacterMovement _characterref) "MOVE_Walking" 0))
          (:else))))))

(event EventBeginPlay
  (bind _asbp_flchar (Utilities|Casting|CastToBP_FLChar (Components|GetOwner)))
  (bind _output_get (Variables|Default|SetCharacterRef _asbp_flchar))
  (Variables|Default|SetFollowCamera (Variables|/Script/FirstLight.FirstLightPlayerCharacter|GetFollowCamera _output_get))
  (Variables|Default|SetAttackSystem (Variables|/Game/FirstLight/Characters/BP_FLChar.BP_FLChar_C|GetBP_AttackSystem _output_get)))

(event Input|KeyboardEvents|DebugKeyH
  (params (Key :type Key%20Structure :default "None") (ActionValue :type Input%20Action%20Value%20Structure))
  ;[0.05127 0.05127 0.05127] Pickup Trace
  (:Pressed
    (for _array_element (Variables|Default|GetWeaponSlots)
      (Development|PrintString (Utilities|String|ToString(Name) (.rowname (.item _array_element)))))))

(fn AddWeapontoInventory
  (params (NewItem :type S%20UI%20Equipment%20Slot%20Structure%20%28by%20ref%29))
  (Utilities|Array|Add (Variables|Default|GetWeaponSlots) NewItem))

(fn EquipWeapon
  (params (EquipmentToAdd :type S%20UI%20Equipment%20Slot%20Structure))
  (Default|EquipItem (Variables|Default|GetCharacterRef) EquipmentToAdd))