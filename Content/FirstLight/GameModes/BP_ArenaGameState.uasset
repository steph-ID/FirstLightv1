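; Game state for the arena mode that tracks living enemies and drives respawning of enemies when none remain.
; On BeginPlay it flags the map as an arena and asks BP_ArenaGameMode to spawn enemies.
; ReduceSpawnedCount decrements the alive count, prints it, and runs CheckEnemiesLeft, which calls the game mode's spawn again when the count reaches zero.
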(event `self.ReceiveBeginPlay`
  (set `self.ArenaMap` true)
  (bind _asbp_arena_game_mode (cast `/Game/FirstLight/GameModes/BP_ArenaGameMode` (`GameplayStatics.GetGameMode`)))
  (`/Game/FirstLight/GameModes/BP_ArenaGameMode.SpawnEnemy` _asbp_arena_game_mode))

(event `CheckEnemiesLeft`
  (if (== (`self.EnemiesAlive`) 0)
    (bind _asbp_arena_game_mode (cast `/Game/FirstLight/GameModes/BP_ArenaGameMode` (`GameplayStatics.GetGameMode`)))
    (`/Game/FirstLight/GameModes/BP_ArenaGameMode.SpawnEnemy` _asbp_arena_game_mode)))

(fn `ReduceSpawnedCount`
  (bind _enemiesalive (`self.EnemiesAlive`))
  (`/Engine/EditorBlueprintResources/StandardMacros.DecrementInt` _enemiesalive
    (:`  `
      (`self.CheckEnemiesLeft`)
      (`KismetSystemLibrary.PrintString` (`KismetStringLibrary.Conv_IntToString` _enemiesalive)))))

(fn `UserConstructionScript`)