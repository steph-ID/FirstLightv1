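; BP_WeaponAbilities gives an animated weapon's owning character two melee abilities: a narrow single-target strike and a 360-degree whirlwind.
; On BeginPlay it finds the character through the weapon's owner and binds both abilities to the player controller's ability slots.
; Each plays a montage whose notify spawns a short-lived box or sphere collision actor, then damages overlapping BP_AI actors.
; Frontal is an empty stub, and the whirlwind effect spawn is disconnected.
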(event `self.ReceiveBeginPlay`
  (bind _asbp_animated_weapon (cast `/Game/FirstLight/Data/Weapons/BP_AnimatedWeapon` (`self.GetOwner`)))
  (bind _asbp_flchar (cast `/Game/FirstLight/Characters/BP_FLChar` (`Actor.GetOwner` _asbp_animated_weapon)))
  (set `self.OwnerCharacter` _asbp_flchar)
  (bind _asbp_flplayer_controller (cast `/Game/FirstLight/Controllers/BP_FirstLightPlayerController` (`GameplayStatics.GetPlayerController` 0)))
  (add `/Game/FirstLight/Controllers/BP_FirstLightPlayerController.Ability1` _asbp_flplayer_controller (delegate `MeleeNarrow`))
  (add `/Game/FirstLight/Controllers/BP_FirstLightPlayerController.Ability2` _asbp_flplayer_controller (delegate `Melee360`)))

(event `MeleeNarrow`
  (bind _ownercharacter (`self.OwnerCharacter`))
  (bind _rootcomponent (`Actor.RootComponent` _ownercharacter))
  (`|PlayMontage` (`Character.Mesh` _ownercharacter) (`self.Montage to Play`) -0.75 0.0 "Reverse"
    (:`OnNotifyBegin`
      (bind _returnvalue (`|SpawnActorFromClass` "/Game/FirstLight/Data/Weapons/BP_SingleTarget.BP_SingleTarget_C" (`KismetMathLibrary.MakeTransform` (+ (`SceneComponent.K2_GetComponentLocation` _rootcomponent) (0.0 0.0 30.0)) (`KismetMathLibrary.ComposeRotators` (`SceneComponent.K2_GetComponentRotation` _rootcomponent) (struct :`Yaw` -90.0))) "Undefined" "OverrideRootScale" null (struct) (struct) null))
      (`Actor.SetLifeSpan` _returnvalue 0.5)
      (`self.ApplyDamageToActors` (`/Game/FirstLight/Data/Weapons/BP_SingleTarget.Box` _returnvalue)))))

(event `Melee360`
  (bind _ownercharacter (`self.OwnerCharacter`))
  (bind _returnvalue_location (`KismetMathLibrary.BreakTransform` (`Actor.GetTransform` _ownercharacter)))
  (set `self.DamageRadius` 10.0)
  (`|PlayMontage` (`Character.Mesh` _ownercharacter) "/Game/StylizedCharacter/Animations/Character/Human/Female/Old_Montages/A_Hu_F_Combat_Whirlwind_Montage_Skill.A_Hu_F_Combat_Whirlwind_Montage_Skill"
    (:`OnNotifyBegin`
      (bind _returnvalue (`|SpawnActorFromClass` "/Game/FirstLight/Data/Weapons/BP_AoE_Collision.BP_AoE_Collision_C" (`KismetMathLibrary.MakeTransform` (+ _returnvalue_location (0.0 0.0 30.0)) (struct) (* (1.0 1.0 1.0) (`self.DamageRadius`))) "AlwaysSpawn" "OverrideRootScale" _ownercharacter (`GameplayStatics.GetPlayerPawn` 0)))
      (`Actor.SetLifeSpan` _returnvalue 0.5)
      (`self.ApplyDamageToActors` (`/Game/FirstLight/Data/Weapons/BP_AoE_Collision.Sphere` _returnvalue)))))

(event `Frontal`)

(fn `ApplyDamageToActors`
  (params (OverlappedComponent :type "PrimitiveComponent Object Reference"))
  (for _array_element (`PrimitiveComponent.GetOverlappingActors` OverlappedComponent "/Game/FirstLight/AI/Test/BP_AI.BP_AI_C")
    (`GameplayStatics.ApplyDamage` _array_element (`self.Damage`) (`GameplayStatics.GetPlayerController` 0) (`self.OwnerCharacter`))))