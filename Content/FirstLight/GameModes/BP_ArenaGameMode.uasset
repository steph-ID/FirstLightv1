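; BP_ArenaGameMode is the FirstLight arena game mode Blueprint, mostly unwired in its current state.
; A level-loaded handler has player controller 0 create its HUD, but its only binding sits in unreachable nodes.
; Those disconnected nodes also load the Arena level instance, create a player and conditionally start a new arena game.
; BeginPlay is empty, and the match-state event only sets NewState to Waiting.
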(event `self.ReceiveBeginPlay`)

(event `OnLevelLoaded_Event`
  (bind _asbp_first_light_player_controller (cast `/Game/FirstLight/Controllers/BP_FirstLightPlayerController` (`GameplayStatics.GetPlayerController` 0)))
  (`/Game/FirstLight/Controllers/BP_FirstLightPlayerController.CreatePlayerHUD` _asbp_first_light_player_controller))

(event `self.K2_OnSetMatchState`
  (params (NewState :type Name))
  (set `self.New State` "Waiting"))

(fn `UserConstructionScript`)