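; Melee attack component for BP_FLChar, with montage attack events, combo state and weapon hit detection.
; Timer-driven loops either sphere-trace between weapon points or overlap the owner's capsule to damage BP_AI.
; Throttled hits add camera shake, sound and blood.
; The combo is only partly wired: the AttackIndex dispatch is disconnected and IA_Attack completion only resets the combo.
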(event `self.ReceiveBeginPlay`
  (bind _asbp_flchar (cast `/Game/FirstLight/Characters/BP_FLChar` (`self.GetOwner`)))
  (bind _output_get (set `self.CharacterBP` _asbp_flchar))
  (set `self.CharacterMesh` (`Character.Mesh` _output_get)))

(event `EnhancedInput|/Game/FirstLight/Characters/Input/Actions/IA_Attack`
  (params (ActionValue :type Boolean) (ElapsedSeconds :type "Float (double-precision)") (TriggeredSeconds :type "Float (double-precision)") (InputAction :type "InputAction Object Reference" :default "/Game/FirstLight/Characters/Input/Actions/IA_Attack.IA_Attack"))
  ;[0.05127 0.05127 0.05127] Attack Input
  (:`Completed`
    (`self.StopCombo`)))

(event `Attack1`
  ;[0.05127 0.05127 0.05127] Attack 1
  (`/Engine/EditorBlueprintResources/StandardMacros.DoOnce` false :!label _label
    (:`Completed`
      (`KismetSystemLibrary.Delay` 0.2)
      (`SkeletalMeshComponent.PlayAnimation` (`self.CharacterMesh`) (`self.Montage to Play`) false)
      (`/Engine/EditorBlueprintResources/StandardMacros.IncrementInt` (`self.AttackIndex`)
        (:`  `
          (goto _label :!via `Reset`))))))

(event `PrimaryAttack`
  ;[0.05127 0.05127 0.05127] Primary Attack
  (if (`self.IsAttacking`)
    (set `self.SaveAttack` true)
    (else
      (set `self.IsAttacking` true))))

(event `Attack2`
  ;[0.05127 0.05127 0.05127] Attack 2
  (`/Engine/EditorBlueprintResources/StandardMacros.DoOnce` false :!label _label_2
    (:`Completed`
      (`KismetSystemLibrary.Delay` 0.2)
      (`|PlayMontage` (`self.CharacterMesh`) "/Game/StylizedCharacter/Animations/Character/Human/Female/Montages/A_Hu_F_Combat_1H_Attack01_Montage.A_Hu_F_Combat_1H_Attack01_Montage"
        (:`then`
          (`/Engine/EditorBlueprintResources/StandardMacros.IncrementInt` (`self.AttackIndex`)
            (:`  `
              (goto _label_2 :!via `Reset`))))))))

(event `AttackCombo`
  ;[0.05127 0.05127 0.05127] Continue Attack Combo
  (if (`self.SaveAttack`)
    (set `self.SaveAttack` false)
    (else
      (`self.StopCombo`))))

(event `Attack3`
  ;[0.05127 0.05127 0.05127] Attack 3
  (`/Engine/EditorBlueprintResources/StandardMacros.DoOnce` false :!label _label_3
    (:`Completed`
      (`KismetSystemLibrary.Delay` 0.2)
      (`|PlayMontage` (`self.CharacterMesh`) "/Game/Kick_Montage.Kick_Montage"
        (:`then`
          (`/Engine/EditorBlueprintResources/StandardMacros.IncrementInt` (`self.AttackIndex`)
            (:`  `
              (goto _label_3 :!via `Reset`))))))))

(event `StopCombo`
  ;[0.05127 0.05127 0.05127] Stop Attack/Combo
  (set `self.IsAttacking` false)
  (set `self.AttackIndex` 0))

(event `Attack4`
  ;[0.05127 0.05127 0.05127] Attach 4
  (`/Engine/EditorBlueprintResources/StandardMacros.DoOnce` false :!label _label_4
    (:`Completed`
      (`KismetSystemLibrary.Delay` 0.2)
      (`|PlayMontage` (`self.CharacterMesh`) "/Game/StylizedCharacter/Animations/Character/Human/Female/Montages/A_Hu_F_Combat_1H_Attack02_Montage.A_Hu_F_Combat_1H_Attack02_Montage"
        (:`then`
          (`/Engine/EditorBlueprintResources/StandardMacros.IncrementInt` (`self.AttackIndex`)
            (:`  `
              (goto _label_4 :!via `Reset`))))))))

(event `StartSwordTrace`
  ;[0.05127 0.05127 0.05127] Sword Trace
  (bind _returnvalue (`KismetSystemLibrary.K2_SetTimerDelegate` (delegate `SwordTraceLoop`) 0.001 true))
  (set `self.SwordTraceLoopTimer` _returnvalue))

(event `SphereTrace`
  ;[0.05127 0.05127 0.05127] Sphere Trace (Stab & Kick)
)

(event `SwordTraceLoop`
  (bind _capsulecomponent (`Character.CapsuleComponent` (`self.CharacterBP`)))
  ;[0.05127 0.05127 0.05127] Sword Trace
  (bind (_outactors _returnvalue) (`KismetSystemLibrary.ComponentOverlapActors` _capsulecomponent (`SceneComponent.K2_GetComponentToWorld` _capsulecomponent) (`|MakeArray` "ObjectTypeQuery3" :!type "EObjectTypeQuery Enum") "/Game/FirstLight/AI/BP_AI.BP_AI_C"))
  (for _array_element _outactors
    (if _returnvalue
      (`/Engine/EditorBlueprintResources/StandardMacros.DoOnce` false :!label _label_5
        (:`Completed`
          (`GameplayStatics.ApplyDamage` _array_element 10.0)
          (bind (_returnvalue_bblockinghit _returnvalue_binitialoverlap _returnvalue_time _returnvalue_distance _returnvalue_location _returnvalue_impactpoint _returnvalue_normal) (`GameplayStatics.BreakHitResult` (`GameplayStatics.MakeHitResult` false _returnvalue)))
          (`GameplayStatics.PlayWorldCameraShake` "/Game/FirstLight/Blueprints/BP_SwordHitCameraShake.BP_SwordHitCameraShake_C" _returnvalue_location 0.0 2000.0)
          (`self.PlaySwordHitSounds`)
          (`GameplayStatics.SpawnEmitterAtLocation` "/Game/Realistic_Starter_VFX_Pack_Vol2/Particles/Blood/P_Blood_Splat_Cone.P_Blood_Splat_Cone" _returnvalue_location (`KismetMathLibrary.MakeRotFromXY` _returnvalue_normal _returnvalue_normal) (0.4 0.4 0.4) true "AutoRelease")
          (`KismetSystemLibrary.Delay` 0.5)
          (goto _label_5 :!via `Reset`))))))

(event `StopSwordTrace`
  ;[0.05127 0.05127 0.05127] Sword Trace
  (`KismetSystemLibrary.K2_ClearAndInvalidateTimerHandle` (`self.SwordTraceLoopTimer`)))

(event `PlaySwordHitSounds`
  ;[0.05127 0.05127 0.05127] Sword Hit Sounds
  (`GameplayStatics.PlaySoundAtLocation` "/Game/FirstLight/Audio/SwordHits/MS_SwordHit.MS_SwordHit" (`Actor.K2_GetActorLocation` (`self.GetOwner`)) (struct) 1.0 1.0 0.0 null null null null))

(event `StopWeaponTrace`
  ;[0.05127 0.05127 0.05127] Weapon Trace
  (`KismetSystemLibrary.K2_ClearAndInvalidateTimerHandle` (`self.WeaponTraceLoopTimer`)))

(event `StartWeaponTrace`
  ;[0.05127 0.05127 0.05127] Weapon Trace
  (bind _returnvalue (`KismetSystemLibrary.K2_SetTimerDelegate` (delegate `WeaponTraceLoop`) 0.001 true))
  (set `self.WeaponTraceLoopTimer` _returnvalue))

(event `WeaponTraceLoop`
  (bind _characterbp (`self.CharacterBP`))
  ;[0.05127 0.05127 0.05127] Weapon Trace
  (bind (_outhit _returnvalue) (`KismetSystemLibrary.SphereTraceSingle` :`Start` (`SceneComponent.K2_GetComponentLocation` (`/Game/FirstLight/Characters/BP_FLChar.WeaponTopPoint` _characterbp)) :`End` (`SceneComponent.K2_GetComponentLocation` (`/Game/FirstLight/Characters/BP_FLChar.WeaponBottomPoint` _characterbp)) :`Radius` 20.0 :`TraceChannel` "TraceTypeQuery1" :`DrawDebugType` "ForDuration" :`DrawTime` (`self.Draw Time`)))
  (if _returnvalue
    (bind (_bblockinghit _binitialoverlap _time _distance _location _impactpoint _normal _impactnormal _physmat _hitactor) (`GameplayStatics.BreakHitResult` _outhit))
    (`/Engine/EditorBlueprintResources/StandardMacros.IsValid` _hitactor
      (:`Is Valid`
        (if (`Actor.ActorHasTag` _hitactor "Damageable")
          (`/Engine/EditorBlueprintResources/StandardMacros.DoOnce` false :!label _label_6
            (:`Completed`
              (bind _asbp_ai (cast `/Game/FirstLight/AI/BP_AI` _hitactor))
              (`/Game/FirstLight/AI/BP_AI.HandleDamage` _asbp_ai (`GameplayStatics.GetPlayerController` 0))
              (`GameplayStatics.PlayWorldCameraShake` "/Game/FirstLight/Blueprints/BP_SwordHitCameraShake.BP_SwordHitCameraShake_C" _location 0.0 5000.0)
              (`self.PlaySwordHitSounds`)
              (`GameplayStatics.SpawnEmitterAtLocation` "/Game/Realistic_Starter_VFX_Pack_Vol2/Particles/Blood/P_Blood_Splat_Cone.P_Blood_Splat_Cone" _location (`KismetMathLibrary.MakeRotFromXY` _normal _normal) (0.4 0.4 0.4) true "AutoRelease")
              (`KismetSystemLibrary.Delay` 0.5)
              (goto _label_6 :!via `Reset`))))))))

(fn `PlayWeaponHitSound`
  (`GameplayStatics.PlaySoundAtLocation` (`self.WeaponHitSound`) (`Actor.K2_GetActorLocation` (`self.GetOwner`)) (struct) 1.0 1.0 0.0 null null null null))