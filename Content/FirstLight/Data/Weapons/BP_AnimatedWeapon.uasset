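; Melee weapon actor that sets its static and skeletal meshes from an item data table row on construction.
; Between start and stop events, a fast looping timer sphere-traces between top and bottom blade points, with debug drawing.
; Hits on "Damageable" actors apply damage, camera shake, sound and blood particles, gated by a DoOnce that resets after a short delay.
; Two ability events forward to BPWeaponAbilities for narrow and 360 melee attacks.
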(event `self.ReceiveBeginPlay`
  (bind _asbp_flchar (cast `/Game/FirstLight/Characters/BP_FLChar` (`self.GetOwner`)))
  (set `self.OwnerCharacter` _asbp_flchar))

(event `StartWeaponTrace`
  (bind _returnvalue (`KismetSystemLibrary.K2_SetTimerDelegate` (delegate `WeaponTraceLoop`) 0.001 true))
  (set `self.WeaponTraceLoopTimer` _returnvalue))

(event `WeaponTraceLoop`
  (bind (_outhit _returnvalue) (`KismetSystemLibrary.SphereTraceSingle` (`SceneComponent.K2_GetComponentLocation` (`self.WeaponActiveTop`)) (`SceneComponent.K2_GetComponentLocation` (`self.WeaponActiveBottom`)) 15.0 "TraceTypeQuery1" false (`|MakeArray` (`self.GetOwner`)) "ForDuration" true (struct :`R` 1.0 :`A` 1.0) (struct :`G` 1.0 :`A` 1.0) (`self.DrawTime`)))
  (if _returnvalue
    (bind (_bblockinghit _binitialoverlap _time _distance _location _impactpoint _normal _impactnormal _physmat _hitactor) (`GameplayStatics.BreakHitResult` _outhit))
    (if (`self.ActorHasTag` _hitactor "Damageable")
      (`/Engine/EditorBlueprintResources/StandardMacros.DoOnce` false :!label _label
        (:`Completed`
          (`GameplayStatics.ApplyDamage` _hitactor 10.0 null (`self.GetOwner`))
          (`GameplayStatics.PlayWorldCameraShake` "/Game/FirstLight/Blueprints/BP_SwordHitCameraShake.BP_SwordHitCameraShake_C" _location 0.0 2000.0)
          (`self.PlayWeaponHitSound`)
          (`GameplayStatics.SpawnEmitterAtLocation` "/Game/Realistic_Starter_VFX_Pack_Vol2/Particles/Blood/P_Blood_Splat_Cone.P_Blood_Splat_Cone" _location (`KismetMathLibrary.MakeRotFromXY` _normal _normal) (0.4 0.4 0.4) true "AutoRelease")
          (`KismetSystemLibrary.Delay` 0.5)
          (goto _label :!via `Reset`))))))

(event `StopWeaponTrace`
  (`KismetSystemLibrary.K2_ClearAndInvalidateTimerHandle` (`self.WeaponTraceLoopTimer`)))

(event `Ability1`
  (`/Game/FirstLight/Data/Weapons/BP_WeaponAbilities.MeleeNarrow` (`self.BP_WeaponAbilities`)))

(event `Ability2`
  (`/Game/FirstLight/Data/Weapons/BP_WeaponAbilities.Melee360` (`self.BP_WeaponAbilities`)))

(fn `ChangeWeapon`
  (bind _itemdata (`self.ItemData`))
  (bind _returnvalue (`|GetDataTableRow` (break `DataTableRowHandle` (break `/Game/FirstLight/Data/Common/S_UIEquipmentSlot` _itemdata)) (`.RowName` (break `DataTableRowHandle` (break `/Game/FirstLight/Data/Common/S_UIEquipmentSlot` _itemdata))))
    (:`then`
      (bind (_name _type _class _icon _staticmesh _skeletalmesh) (break `/Game/FirstLight/Data/Weapons/S_Weapons` _returnvalue))
      (`StaticMeshComponent.SetStaticMesh` (`self.StaticMesh`) _staticmesh)
      (`SkeletalMeshComponent.SetSkeletalMeshAsset` (`self.SkeletalMesh`) _skeletalmesh)
      (`SceneComponent.K2_SetRelativeLocation` (`self.WeaponActiveTop`) (`KismetMathLibrary.MakeVector` 0.0 (/ (.y (`KismetSystemLibrary.GetComponentBounds` (`self.SkeletalMesh`))) 3.5)) false false))))

(fn `PlayWeaponHitSound`
  (`GameplayStatics.PlaySoundAtLocation` (`self.WeaponHitSound`) (`self.K2_GetActorLocation` (`self.GetOwner`)) (struct) 1.0 1.0 0.0 null null null null))

(fn `UserConstructionScript`
  (`self.ChangeWeapon`))