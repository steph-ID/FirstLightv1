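; Test dummy character for trying out combat hits and stealth back assassinations, with health bar and execute-prompt widgets turned toward the player camera.
; Damage plays a random hit montage and grunt, launches the dummy along the player's facing, and lowers BPPlayerStats health, ragdolling on death.
; An overlap radius toggles the execute prompt.
; StealthBackAssassin plays the paired victim montage, starts a delayed ragdoll, and returns alignment location and rotation.
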(event `self.ReceiveBeginPlay`
  (bind _aswbp_enemy_health_bar (cast `/Game/FirstLight/Blueprints/UI/InWorldText/WBP_EnemyHealthBar` (`WidgetComponent.GetWidget` (`self.HealthBarWidget`))))
  (set `self.EnemyHealthBarUI` _aswbp_enemy_health_bar))

(event `self.ReceiveTick`
  (params (DeltaSeconds :type "Float (single-precision)"))
  (`SceneComponent.K2_SetWorldRotation` (`self.ExecuteWidget`) (`KismetMathLibrary.FindLookAtRotation` (`SceneComponent.K2_GetComponentLocation` (`self.ExecuteWidget`)) (`SceneComponent.K2_GetComponentLocation` (`PlayerCameraManager.TransformComponent` (`GameplayStatics.GetPlayerCameraManager` 0)))) false false)
  (`SceneComponent.K2_SetWorldRotation` (`self.HealthBarWidget`) (`KismetMathLibrary.FindLookAtRotation` (`SceneComponent.K2_GetComponentLocation` (`self.ExecuteWidget`)) (`SceneComponent.K2_GetComponentLocation` (`PlayerCameraManager.TransformComponent` (`GameplayStatics.GetPlayerCameraManager` 0)))) false false))

(event `self.ReceiveAnyDamage`
  (params (Damage :type "Float (single-precision)") (DamageType :type "DamageType Object Reference") (InstigatedBy :type "Controller Object Reference") (DamageCauser :type "Actor Object Reference"))
  (bind _hitanims (`self.HitAnims`))
  (`self.PlayAnimMontage` (`|GetArrayItem` _hitanims (`KismetMathLibrary.RandomIntegerInRange` 0 (- (`KismetArrayLibrary.Array_Length` _hitanims) 1))))
  (bind _asbp_character_base (cast `/Game/FirstLight/Characters/Tests/BP_CharacterBase` (`GameplayStatics.GetPlayerCharacter` 0)))
  (`self.LaunchCharacter` (* (`KismetMathLibrary.GetForwardVector` (`self.K2_GetActorRotation` _asbp_character_base)) 700.0))
  (`GameplayStatics.PlaySoundAtLocation` "/Game/FirstLight/Audio/Deaths/416839__tonsil5__grunt1-death-pain.416839__tonsil5__grunt1-death-pain" (`self.K2_GetActorLocation`) (struct) 1.0 (`KismetMathLibrary.RandomFloatInRange` 1.0 1.3) 0.0 null null null null)
  (bind _isdead (`/Game/FirstLight/Blueprints/CharacterComponents/BPC_CharacterAttributes.DecreaseHealth` (`self.BP_PlayerStats`) Damage))
  (if _isdead
    (`PrimitiveComponent.SetSimulatePhysics` (`self.Mesh`) true)
    (`GameplayStatics.PlaySoundAtLocation` "/Game/FirstLight/Audio/Deaths/SC_M_Death.SC_M_Death" (`self.K2_GetActorLocation`) (struct) 1.0 1.0 0.0 null null null null)))

(event `Ragdoll`
  ;[0.05127 0.05127 0.05127] Ragdoll
  (`KismetSystemLibrary.Delay` 2.5)
  (`PrimitiveComponent.SetSimulatePhysics` (`self.Mesh`) true))

(event `self.ExecuteRadius.OnComponentBeginOverlap`
  (params (OverlappedComponent :type "PrimitiveComponent Object Reference") (OtherActor :type "Actor Object Reference") (OtherComp :type "PrimitiveComponent Object Reference") (OtherBodyIndex :type Integer) (bFromSweep :type Boolean) (SweepResult :type "HitResult Structure (by ref)"))
  (cast `/Game/FirstLight/Characters/Tests/BP_CharacterBase` OtherActor)
  (`SceneComponent.SetVisibility` (`self.ExecuteWidget`) true false))

(event `self.ExecuteRadius.OnComponentEndOverlap`
  (params (OverlappedComponent :type "PrimitiveComponent Object Reference") (OtherActor :type "Actor Object Reference") (OtherComp :type "PrimitiveComponent Object Reference") (OtherBodyIndex :type Integer))
  (cast `/Game/FirstLight/Characters/Tests/BP_CharacterBase` OtherActor)
  (`SceneComponent.SetVisibility` (`self.ExecuteWidget`) false false))

(fn `StealthBackAssassin`
  (returns (ReferenceLocation :type "Vector Structure") (KillRotation :type "Rotator Structure"))
  (`self.PlayAnimMontage` "/Game/FirstLight/Characters/Animations/Attacks/Paired_Knife_Stealth_KidneyAndNeck_Vic_Montage.Paired_Knife_Stealth_KidneyAndNeck_Vic_Montage")
  (`self.Ragdoll`)
  (`SceneComponent.SetVisibility` (`self.ExecuteWidget`) false false)
  (return (`SceneComponent.K2_GetComponentLocation` (`self.KillReference`)) (`self.K2_GetActorRotation`)))

(fn `UserConstructionScript`)