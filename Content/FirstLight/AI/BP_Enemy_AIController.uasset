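; AI controller for enemies that runs the BT_AI behavior tree on BeginPlay and supplies its chase target.
; AI Perception updates drive the TargetActor blackboard key: a successful sight stimulus stores the sensed actor.
; Stimuli from any other sense clear the key, while losing sight leaves it unchanged.
; The Possess event is empty, with an unused ability-system attribute lookup left in the graph.
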(event `self.ReceiveBeginPlay`
  (`self.RunBehaviorTree` "/Game/FirstLight/AI/BT_AI.BT_AI"))

(event `self.AIPerception.OnTargetPerceptionUpdated`
  (params (Actor :type "Actor Object Reference") (Stimulus :type "AIStimulus Structure"))
  ;[0.05127 0.05127 0.05127] Detect & Chase Target
  (bind _returnvalue (`AIPerceptionSystem.GetSenseClassForStimulus` Stimulus))
  (if (== _returnvalue "/Script/AIModule.AISense_Sight")
    (if (`.bSuccessfullySensed` (break `AIStimulus` Stimulus))
      (`BlackboardComponent.SetValueAsObject` (`AIBlueprintHelperLibrary.GetBlackboard` null) "TargetActor" Actor))
    (else
      (`BlackboardComponent.SetValueAsObject` (`AIBlueprintHelperLibrary.GetBlackboard` null) "TargetActor" null))))

(event `self.ReceivePossess`
  (params (PossessedPawn :type "Pawn Object Reference")))

(fn `UserConstructionScript`)