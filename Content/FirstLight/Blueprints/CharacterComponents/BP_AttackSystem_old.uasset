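; Player attack component that runs a four-step melee montage combo on the owning BP_FL_PlayerCharacter.
; IA_Attack starts an attack or buffers input while attacking; AttackCombo then plays the step at AttackIndex or resets the combo.
; SphereTrace damages "Damageable" actors with camera shake, sound and blood effects.
; The timer-driven sword trace loop is empty, as its sweep logic is disconnected.
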(event `self.ReceiveBeginPlay`
  (bind _asbp_fl_player_character (cast `/Game/FirstLight/Characters/BP_FL_PlayerCharacter` (`self.GetOwner`)))
  (bind _output_get (set `self.CharacterBP` _asbp_fl_player_character))
  (set `self.CharacterMesh` (`Character.Mesh` _output_get)))

(event `EnhancedInput|/Game/FirstLight/Characters/Input/Actions/IA_Attack`
  (params (ActionValue :type Boolean) (ElapsedSeconds :type "Float (double-precision)") (TriggeredSeconds :type "Float (double-precision)") (InputAction :type "InputAction Object Reference" :default "/Game/FirstLight/Characters/Input/Actions/IA_Attack.IA_Attack"))
  ;[0.05127 0.05127 0.05127] Combo System
  ;;[0.05127 0.05127 0.05127] Attack Input
  (:`Started`
    (if (`self.CanAttack`)
      (`self.PrimaryAttack`))))

(event `Attack1`
  ;[0.05127 0.05127 0.05127] Combo System
  ;;[0.05127 0.05127 0.05127] Attack 1
  (`/Engine/EditorBlueprintResources/StandardMacros.DoOnce` false :!label _label
    (:`Completed`
      (`KismetSystemLibrary.Delay` 0.2)
      (`|PlayMontage` (`self.CharacterMesh`) "/Game/FirstLight/Characters/Animations/Attacks/Sword/Attack1_Montage.Attack1_Montage"
        (:`then`
          (`/Engine/EditorBlueprintResources/StandardMacros.IncrementInt` (`self.AttackIndex`)
            (:`  `
              (goto _label :!via `Reset`))))))))

(event `PrimaryAttack`
  ;[0.05127 0.05127 0.05127] Combo System
  ;;[0.05127 0.05127 0.05127] Primary Attack
  (if (`self.IsAttacking`)
    (set `self.SaveAttack` true)
    (else
      (set `self.IsAttacking` true)
      (switch `int` (`self.AttackIndex`) :!label _label_2
        (:`0`
          (`self.Attack1`))
        (:`1`
          (`self.Attack2`))
        (:`2`
          (`self.Attack3`))
        (:`3`
          (`self.Attack4`))))))

(event `Attack2`
  ;[0.05127 0.05127 0.05127] Combo System
  ;;[0.05127 0.05127 0.05127] Attack 2
  (`/Engine/EditorBlueprintResources/StandardMacros.DoOnce` false :!label _label_3
    (:`Completed`
      (`KismetSystemLibrary.Delay` 0.2)
      (`|PlayMontage` (`self.CharacterMesh`) "/Game/FirstLight/Characters/Animations/Attacks/Sword/Attack2_Montage.Attack2_Montage"
        (:`then`
          (`/Engine/EditorBlueprintResources/StandardMacros.IncrementInt` (`self.AttackIndex`)
            (:`  `
              (goto _label_3 :!via `Reset`))))))))

(event `AttackCombo`
  ;[0.05127 0.05127 0.05127] Combo System
  ;;[0.05127 0.05127 0.05127] Continue Attack Combo
  (if (`self.SaveAttack`)
    (set `self.SaveAttack` false)
    (goto _label_2)
    (else
      (`self.StopCombo`))))

(event `Attack3`
  ;[0.05127 0.05127 0.05127] Combo System
  ;;[0.05127 0.05127 0.05127] Attack 3
  (`/Engine/EditorBlueprintResources/StandardMacros.DoOnce` false :!label _label_4
    (:`Completed`
      (`KismetSystemLibrary.Delay` 0.2)
      (`|PlayMontage` (`self.CharacterMesh`) "/Game/FirstLight/Characters/Animations/Attacks/Sword/Kick_Montage.Kick_Montage"
        (:`then`
          (`/Engine/EditorBlueprintResources/StandardMacros.IncrementInt` (`self.AttackIndex`)
            (:`  `
              (goto _label_4 :!via `Reset`))))))))

(event `StopCombo`
  ;[0.05127 0.05127 0.05127] Combo System
  ;;[0.05127 0.05127 0.05127] Stop Attack/Combo
  (set `self.IsAttacking` false)
  (set `self.AttackIndex` 0))

(event `Attack4`
  ;[0.05127 0.05127 0.05127] Combo System
  ;;[0.05127 0.05127 0.05127] Attach 4
  (`/Engine/EditorBlueprintResources/StandardMacros.DoOnce` false :!label _label_5
    (:`Completed`
      (`KismetSystemLibrary.Delay` 0.2)
      (`|PlayMontage` (`self.CharacterMesh`) "/Game/FirstLight/Characters/Animations/Attacks/Sword/Attack3_Montage.Attack3_Montage"
        (:`then`
          (`/Engine/EditorBlueprintResources/StandardMacros.IncrementInt` (`self.AttackIndex`)
            (:`  `
              (goto _label_5 :!via `Reset`))))))))

(event `StartSwordTrace`
  ;[0.05127 0.05127 0.05127] Sword Trace
  (bind _returnvalue (`KismetSystemLibrary.K2_SetTimerDelegate` (delegate `SwordTraceLoop`) 0.001 true))
  (set `self.SwordTraceLoopTimer` _returnvalue))

(event `SphereTrace`
  (bind _returnvalue (`SceneComponent.K2_GetComponentLocation` (`/Game/FirstLight/Characters/BP_CharacterBase.SphereTrace` (`self.CharacterBP`))))
  ;[0.05127 0.05127 0.05127] Sphere Trace (Stab & Kick)
  (bind (_outhit _returnvalue_2) (`KismetSystemLibrary.SphereTraceSingle` :`Start` _returnvalue :`End` _returnvalue :`Radius` 25.0 :`TraceChannel` "TraceTypeQuery1" :`DrawTime` (`self.Draw Time`)))
  (if _returnvalue_2
    (bind (_bblockinghit _binitialoverlap _time _distance _location _impactpoint _normal _impactnormal _physmat _hitactor) (`GameplayStatics.BreakHitResult` _outhit))
    (if (`Actor.ActorHasTag` _hitactor "Damageable")
      (`GameplayStatics.ApplyDamage` _hitactor 10.0)
      (`GameplayStatics.PlayWorldCameraShake` "/Game/FirstLight/Blueprints/BP_SwordHitCameraShake.BP_SwordHitCameraShake_C" _location 0.0 2000.0)
      (`self.PlaySwordHitSounds`)
      (`GameplayStatics.SpawnEmitterAtLocation` "/Game/Realistic_Starter_VFX_Pack_Vol2/Particles/Blood/P_Blood_Splat_Cone.P_Blood_Splat_Cone" _location (`KismetMathLibrary.MakeRotFromXY` _normal _normal) (0.4 0.4 0.4) true "AutoRelease"))))

(event `SwordTraceLoop`
  ;[0.05127 0.05127 0.05127] Sword Trace
)

(event `StopSwordTrace`
  ;[0.05127 0.05127 0.05127] Sword Trace
  (`KismetSystemLibrary.K2_ClearAndInvalidateTimerHandle` (`self.SwordTraceLoopTimer`)))

(event `PlaySwordHitSounds`
  ;[0.05127 0.05127 0.05127] Sword Hit Sounds
  (`GameplayStatics.PlaySoundAtLocation` "/Game/FirstLight/Audio/SwordHits/MS_SwordHit.MS_SwordHit" (`Actor.K2_GetActorLocation` (`self.GetOwner`)) (struct) 1.0 1.0 0.0 null null null null))