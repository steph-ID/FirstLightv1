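; Base Blueprint for AI enemy NPCs that carries an overhead health bar widget.
; On BeginPlay it casts the health bar component's widget to WBP_EnemyHealthBar and stores the reference.
; Every Tick it rotates the health bar in world space to face the player camera, acting as a billboard.
; SetEnemyData is an empty function, and the construction script adds no logic.
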(event `self.ReceiveBeginPlay`
  (bind _aswbp_enemy_health_bar (cast `/Game/FirstLight/UI/InWorldText/WBP_EnemyHealthBar` (`WidgetComponent.GetWidget` (`self.HealthBarWidget`))))
  (set `self.EnemyHealthWidget` _aswbp_enemy_health_bar))

(event `self.ReceiveTick`
  (params (DeltaSeconds :type "Float (single-precision)"))
  (`SceneComponent.K2_SetWorldRotation` (`self.HealthBarWidget`) (`KismetMathLibrary.FindLookAtRotation` (`SceneComponent.K2_GetComponentLocation` (`self.HealthBarWidget`)) (`SceneComponent.K2_GetComponentLocation` (`PlayerCameraManager.TransformComponent` (`GameplayStatics.GetPlayerCameraManager` 0)))) false false))

(fn `SetEnemyData`)

(fn `UserConstructionScript`)