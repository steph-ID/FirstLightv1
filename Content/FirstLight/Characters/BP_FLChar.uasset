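; FirstLight character built from modular skeletal mesh parts, handling damage and equipment.
; Construction makes child meshes follow the main mesh's pose and maps them by name as sockets.
; EquipItem reads a data table row, replaces the weapon on that socket with a spawned BP_AnimatedWeapon and attaches it to the matching mesh.
; Damage triggers knockback, grunt and camera shake, then BPCCharacterAttributes reduces health and processes death.
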(event `self.ReceiveBeginPlay`)

(event `self.ReceiveAnyDamage`
  (params (Damage :type "Float (single-precision)") (DamageType :type "DamageType Object Reference") (InstigatedBy :type "Controller Object Reference") (DamageCauser :type "Actor Object Reference"))
  (bind _returnvalue (`self.K2_GetActorLocation`))
  (bind _bpc_characterattributes (`self.BPC_CharacterAttributes`))
  ;[0.05127 0.05127 0.05127] Apply Damage
  (`|ExecutionSequence`
    (:`then_0`
      (`/Engine/EditorBlueprintResources/StandardMacros.IsValid` DamageCauser
        (:`Is Valid`
          (`self.LaunchCharacter` (* (`KismetMathLibrary.GetForwardVector` (`self.K2_GetActorRotation` DamageCauser)) 700.0)))
        (:`Is Not Valid`
          _))
      (`GameplayStatics.PlaySoundAtLocation` "/Game/FirstLight/Audio/Deaths/416839__tonsil5__grunt1-death-pain.416839__tonsil5__grunt1-death-pain" _returnvalue (struct) 1.0 (`KismetMathLibrary.RandomFloatInRange` 1.0 1.3) 0.0 null null null null)
      (`GameplayStatics.PlayWorldCameraShake` "/Game/FirstLight/Blueprints/BP_SwordHitCameraShake.BP_SwordHitCameraShake_C" _returnvalue 0.0 2000.0))
    (:`then_1`
      (bind _isdead (`/Game/FirstLight/Blueprints/CharacterComponents/BPC_CharacterAttributes.DecreaseHealth` _bpc_characterattributes Damage))
      (if _isdead
        (`/Game/FirstLight/Blueprints/CharacterComponents/BPC_CharacterAttributes.ProcessDeath` _bpc_characterattributes)))))

(fn `EquipItem`
  (params (Item :type "/Game/FirstLight/Data/Common/S_UIEquipmentSlot Structure"))
  (bind (_item_datatable _item_rowname) (break `DataTableRowHandle` (break `/Game/FirstLight/Data/Common/S_UIEquipmentSlot` Item)))
  (set `self.EquippedItem` Item)
  (bind _returnvalue (`|GetDataTableRow` _item_datatable _item_rowname)
    (:`then`
      (bind (_name _type _class _icon _staticmesh _skeletalmesh _socket) (break `/Game/FirstLight/Data/Weapons/S_Weapons` _returnvalue))
      (`/Engine/EditorBlueprintResources/StandardMacros.IsValid` _skeletalmesh
        (:`Is Valid`
          (for _array_element (`self.GetAttachedActors` true)
            (bind _asbp_animated_weapon (cast `/Game/FirstLight/Data/Weapons/BP_AnimatedWeapon` _array_element))
            (bind _returnvalue_2 (`|GetEnumeratorNameAsString` _socket))
            (bind _returnvalue_3 (`KismetStringLibrary.Conv_StringToName` _returnvalue_2))
            (if (== (`self.GetAttachParentSocketName` _asbp_animated_weapon) _returnvalue_3)
              (`self.K2_DestroyActor` _array_element)))
          (bind _returnvalue_4 (`|SpawnActorFromClass` "/Game/FirstLight/Data/Weapons/BP_AnimatedWeapon.BP_AnimatedWeapon_C" (`SceneComponent.GetSocketTransform` (`self.CharacterMesh`) _returnvalue_3 "RTS_Component") "Undefined" "OverrideRootScale" self null))
          (`SkeletalMeshComponent.SetSkeletalMeshAsset` (`/Game/FirstLight/Data/Weapons/BP_AnimatedWeapon.SkeletalMesh` _returnvalue_4) _skeletalmesh)
          (`self.K2_AttachToComponent` _returnvalue_4 (`BlueprintMapLibrary.Map_Find` (`self.CharacterSockets`) _returnvalue_2) "None" "KeepRelative" "KeepRelative" "KeepRelative" true))))))

(fn `GetSocketNames`
  (if (`BlueprintMapLibrary.Map_IsEmpty` (`self.CharacterSockets`))
    (for _array_element (`SceneComponent.GetChildrenComponents` (`self.CharacterMesh`) true)
      (bind _asskeletal_mesh_component (cast `SkeletalMeshComponent` _array_element))
      (bind _returnvalue (`KismetSystemLibrary.GetObjectName` _array_element))
      (if (not (`KismetStringLibrary.IsEmpty` _returnvalue))
        (`BlueprintMapLibrary.Map_Add` (`self.CharacterSockets`) _returnvalue _asskeletal_mesh_component)))))

(fn `InitializeCharacterModel`
  (bind _mesh (`self.Mesh`))
  (for _array_element (`SceneComponent.GetChildrenComponents` _mesh true)
    (bind _asskeletal_mesh_component (cast `SkeletalMeshComponent` _array_element))
    (`SkinnedMeshComponent.SetLeaderPoseComponent` _asskeletal_mesh_component _mesh false false)
    (`SkeletalMeshComponent.SetAnimInstanceClass` _mesh (`self.AnimInstanceClass`))))

(fn `RandomizeOutfit`
  (`self.RandomPart` (`self.ChestParts`) (`self.Chest`)))

(fn `RandomPart`
  (params (MeshOptions :type "Array of SkeletalMesh Object Reference (by ref)") (`Part Mesh` :type "SkinnedMeshComponent Object Reference"))
  (bind _output_get (set `self.RandomMesh` (`self.RandomMesh`)))
  (`SkinnedMeshComponent.SetSkinnedAssetAndUpdate` `Part Mesh` _output_get false)
  (for _array_element (`SkeletalMesh.Materials` _output_get)
    (`PrimitiveComponent.SetMaterialByName` `Part Mesh` (`.MaterialSlotName` (break `SkeletalMaterial` _array_element)) (break `SkeletalMaterial` _array_element))))

(fn `UserConstructionScript`
  (set `self.CharacterMesh` (`self.Mesh`))
  (`self.InitializeCharacterModel`)
  (`self.GetSocketNames`))