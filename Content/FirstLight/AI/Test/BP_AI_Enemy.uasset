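; Test AI enemy for an arena mode that chases the player and is tracked in the arena's count of living enemies.
; On BeginPlay it increments EnemiesAlive on BP_ArenaGameState directly, then issues an AI MoveTo toward the first player's BP_FLChar.
; Separate functions raise or lower that count, with the decrease also calling CheckEnemiesLeft; neither is called within this Blueprint.
; The Hit event is empty.
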(event `self.ReceiveBeginPlay`
  (`parent.ReceiveBeginPlay`)
  (bind _asbp_arena_game_state (cast `/Game/FirstLight/GameModes/BP_ArenaGameState` (`GameplayStatics.GetGameState`)))
  (`/Engine/EditorBlueprintResources/StandardMacros.IncrementInt` (`/Game/FirstLight/GameModes/BP_ArenaGameState.EnemiesAlive` _asbp_arena_game_state)
    (:`  `
      (bind _asbp_flchar (cast `/Game/FirstLight/Characters/BP_FLChar` (`GameplayStatics.GetPlayerCharacter` 0)))
      (`|AIMoveTo` self (0.0 0.0 0.0) _asbp_flchar))))

(event `self.ReceiveHit`
  (params (MyComp :type "PrimitiveComponent Object Reference") (Other :type "Actor Object Reference") (OtherComp :type "PrimitiveComponent Object Reference") (bSelfMoved :type Boolean) (HitLocation :type "Vector Structure") (HitNormal :type "Vector Structure") (NormalImpulse :type "Vector Structure") (Hit :type "HitResult Structure (by ref)")))

(fn `IncreaseSpawnedEnemyCount`
  (bind _asbp_arena_game_state (cast `/Game/FirstLight/GameModes/BP_ArenaGameState` (`GameplayStatics.GetGameState`)))
  (`/Engine/EditorBlueprintResources/StandardMacros.IncrementInt` (`/Game/FirstLight/GameModes/BP_ArenaGameState.EnemiesAlive` _asbp_arena_game_state)))

(fn `ReduceSpawnedEnemyCount`
  (bind _asbp_arena_game_state (cast `/Game/FirstLight/GameModes/BP_ArenaGameState` (`GameplayStatics.GetGameState`)))
  (`/Engine/EditorBlueprintResources/StandardMacros.DecrementInt` (`/Game/FirstLight/GameModes/BP_ArenaGameState.EnemiesAlive` _asbp_arena_game_state)
    (:`  `
      (`/Game/FirstLight/GameModes/BP_ArenaGameState.CheckEnemiesLeft` _asbp_arena_game_state))))

(fn `UserConstructionScript`
  (`parent.UserConstructionScript`))